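; BP_TiltingPlatform02 is a platform actor whose Plane tilts while the player's BP_Ball is on it.
; Box overlap begin and end events set IsTilting, responding only to the pawn of player 0.
; Tick uses FInterpTo to ease the Plane's relative roll toward TiltAngle, or back to zero once the ball leaves, with TiltSpeed and DeltaMultiplier controlling the rate.
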(event OnComponentEndOverlap(box)
  (params (OverlappedComponent :type Primitive%20Component%20Object%20Reference) (OtherActor :type Actor%20Object%20Reference) (OtherComp :type Primitive%20Component%20Object%20Reference) (OtherBodyIndex :type Integer))
  (bind _asbp_ball (Utilities|Casting|CastToBP_Ball (Game|Player|GetPlayerPawn 0)))
  (if (== _asbp_ball OtherActor)
    (Variables|Default|SetIsTilting false)))

(event OnComponentBeginOverlap(box)
  (params (OverlappedComponent :type Primitive%20Component%20Object%20Reference) (OtherActor :type Actor%20Object%20Reference) (OtherComp :type Primitive%20Component%20Object%20Reference) (OtherBodyIndex :type Integer) (bFromSweep :type Boolean) (SweepResult :type Hit%20Result%20Structure%20%28by%20ref%29))
  (bind _asbp_ball (Utilities|Casting|CastToBP_Ball (Game|Player|GetPlayerPawn 0)))
  (if (== _asbp_ball OtherActor)
    (Variables|Default|SetIsTilting true)))

(event EventTick
  (params (DeltaSeconds :type Float%20%28single-precision%29))
  (bind _deltamultiplier (Variables|Default|GetDeltaMultiplier))
  (bind _plane (Variables|Default|GetPlane))
  (bind _tiltspeed (Variables|Default|GetTiltSpeed))
  (bind _returnvalue (* DeltaSeconds _deltamultiplier))
  (bind _relativerotation (Variables|/Script/Engine.SceneComponent|GetRelativeRotation _plane))
  (if (Variables|Default|GetIsTilting)
    (Transformation|SetRelativeRotation _plane (Math|Rotator|MakeRotator (Math|Interpolation|FInterpTo (.Roll (Math|Rotator|BreakRotator (Math|Rotator|MakeRotator (.roll _relativerotation) 0.0 0.0))) (Variables|Default|GetTiltAngle) _returnvalue _tiltspeed) 0.0 0.0) false false)
    (else
      (Transformation|SetRelativeRotation _plane (Math|Rotator|MakeRotator (Math|Interpolation|FInterpTo (.roll _relativerotation) 0.0 _returnvalue _tiltspeed) 0.0 0.0) false false))))

(fn ConstructionScript)