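; BP_WinVolume_01 is a level exit trigger that loads Level02 once all crystals are collected.
; When anything begins overlapping its Box, it looks for remaining BP_Crystal_01 and BP_Crystal_02 actors in the world, without filtering the overlapping actor.
; If any remain, it prints a Polish message that not all crystals were collected.
; Otherwise it fades out the player camera, waits for the fade, then opens Level02.
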(event OnComponentBeginOverlap(Box)
  (params (OverlappedComponent :type Primitive%20Component%20Object%20Reference) (OtherActor :type Actor%20Object%20Reference) (OtherComp :type Primitive%20Component%20Object%20Reference) (OtherBodyIndex :type Integer) (bFromSweep :type Boolean) (SweepResult :type Hit%20Result%20Structure%20%28by%20ref%29))
  (bind _outactors (Actor|GetAllActorsOfClass "/Game/blueprints/BP_Crystal_01.BP_Crystal_01_C"))
  (if (> (Utilities|Array|Length _outactors) 0)
    (Development|PrintString "NIE ZEBRANO WSZYSTKICH KRZYSZTAŁÓW" :!label _label)
    (else
      (bind _outactors_2 (Actor|GetAllActorsOfClass "/Game/blueprints/BP_Crystal_02.BP_Crystal_02_C"))
      (if (> (Utilities|Array|Length _outactors_2) 0)
        (goto _label)
        (else
          (CameraFades|StartCameraFade :self (Game|GetPlayerCameraManager 0) :ToAlpha 1.0 :Duration 2.0 :bHoldWhenFinished true)
          (Utilities|FlowControl|Delay 2.0)
          (Game|OpenLevel(byName) "Level02"))))))

(fn ConstructionScript)